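; BP_CameraZone is a placeable trigger volume that switches the player's camera mode while the player is inside.
; On overlap it finds BPC_CameraController on the entering actor and passes itself, its CameraMode Data Asset, rotation and location via EnterZone.
; On exit it calls ExitZone, leaving the controller to choose which camera returns.
; Additional PlayerTrigger-preset shapes merge into one zone, and the preset plus component check filters out NPCs.
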(event `self.ReceiveActorBeginOverlap`
  (params (OtherActor :type "Actor Object Reference"))
  (bind _returnvalue (`self.GetComponentByClass` OtherActor "/Game/SpineTest/CameraSystem/Components/BPC_CameraController.BPC_CameraController_C"))
  ; BP_CameraZone: зона смены камеры.
  ; Вход игрока - старт режима, выход - конец.
  ; Настройка для ЛД: выбрать Camera Mode (Data Asset из CameraSystem/Modes), растянуть ZoneShape (Box Extent) и повернуть актор по стрелке Direction.
  ; Форма зоны: можно добавить любые Box/Sphere/Capsule с пресетом PlayerTrigger, они считаются одной зоной.
  ; Срабатывает только от игрока: пресет PlayerTrigger игнорирует канал NPC, плюс проверка наличия BPC_CameraController у вошедшего актора.
  ;; Вход. Передаём контроллеру камеры: себя, режим, поворот зоны  и позицию зоны.
  (`/Engine/EditorBlueprintResources/StandardMacros.IsValid` _returnvalue
    (:`Is Valid`
      (`/Game/SpineTest/CameraSystem/Components/BPC_CameraController.EnterZone` _returnvalue self (`self.CameraMode`) (`self.K2_GetActorRotation`) (`self.K2_GetActorLocation`)))))

(event `self.ReceiveActorEndOverlap`
  (params (OtherActor :type "Actor Object Reference"))
  (bind _returnvalue (`self.GetComponentByClass` OtherActor "/Game/SpineTest/CameraSystem/Components/BPC_CameraController.BPC_CameraController_C"))
  ; BP_CameraZone: зона смены камеры.
  ; Вход игрока - старт режима, выход - конец.
  ; Настройка для ЛД: выбрать Camera Mode (Data Asset из CameraSystem/Modes), растянуть ZoneShape (Box Extent) и повернуть актор по стрелке Direction.
  ; Форма зоны: можно добавить любые Box/Sphere/Capsule с пресетом PlayerTrigger, они считаются одной зоной.
  ; Срабатывает только от игрока: пресет PlayerTrigger игнорирует канал NPC, плюс проверка наличия BPC_CameraController у вошедшего актора.
  ;; Выход. Контроллер сам решает, какую камеру вернуть: режим предыдущей зоны
  (`/Engine/EditorBlueprintResources/StandardMacros.IsValid` _returnvalue
    (:`Is Valid`
      (`/Game/SpineTest/CameraSystem/Components/BPC_CameraController.ExitZone` _returnvalue self))))

(fn `UserConstructionScript`)