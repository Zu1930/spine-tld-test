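; BP_FollowerNPC is a simple companion NPC that waits for the player to come within an activation radius, then follows permanently.
; A looping timer started on BeginPlay drives the distance checks instead of Tick.
; When the player exceeds follow distance plus a tolerance, the AI controller calls MoveToActor, using follow distance as acceptance radius.
; It skips the call while already moving, so navigation requests are not restarted.
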(event `self.ReceiveBeginPlay`
  ; BP_FollowerNPC: простой компаньон. Ждёт игрока в радиусе ActivationRadius, потом следует за ним и держит дистанцию FollowDistance.
  ;; Запоминаем игрока и запускаем проверку дистанции по таймеру раз в UpdateInterval секунд.
  (set `self.PlayerPawn` (`GameplayStatics.GetPlayerPawn` 0))
  (`KismetSystemLibrary.K2_SetTimerDelegate` (delegate `UpdateFollow`) (`self.UpdateInterval`) true))

(event `UpdateFollow`
  (bind _returnvalue (`self.GetDistanceTo` (`self.PlayerPawn`)))
  ; BP_FollowerNPC: простой компаньон. Ждёт игрока в радиусе ActivationRadius, потом следует за ним и держит дистанцию FollowDistance.
  ;; Активация. NPC стоит на месте, пока игрок не подойдёт ближе ActivationRadius.
  ;; После первой встречи Is Active = true, и дальше NPC следует всегда.
  (`/Engine/EditorBlueprintResources/StandardMacros.IsValid` (`self.PlayerPawn`)
    (:`Is Valid`
      (if (or (`self.bIsActive`) (< _returnvalue (`self.ActivationRadius`)))
        (set `self.bIsActive` true)
        ;; Нужно ли идти. Идём, только если игрок дальше FollowDistance + 50 см.
        (if (> _returnvalue (+ (`self.FollowDistance`) (`self.DistanceTolerance`)))
          ;; Движение к игроку по навмешу через стандартный AIController.
          ;; Не перезапускаем движение, если NPC уже идёт
          ;; Acceptance Radius = FollowDistance - NPC останавливается на комфортной дистанции.
          (bind _asaicontroller (cast `AIController` (`self.GetController`)))
          (if (`|EnumInequality` (`AIController.GetMoveStatus` _asaicontroller) "Moving")
            (`AIController.MoveToActor` _asaicontroller (`self.PlayerPawn`) (`self.FollowDistance`) true true false null true)))))))

(fn `UserConstructionScript`)